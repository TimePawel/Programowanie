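; BP_Crystal is a collectable crystal that spins in place and is absorbed by the player on touch.
; Tick adds a fixed yaw step each frame, and a sphere overlap by the player pawn stores the starting location, scale and light intensity.
; A timeline then pulls it toward the player's current position while shrinking it and fading its point light, destroying the actor when finished.
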(event OnComponentBeginOverlap(Sphere)
  (params (OverlappedComponent :type Primitive%20Component%20Object%20Reference) (OtherActor :type Actor%20Object%20Reference) (OtherComp :type Primitive%20Component%20Object%20Reference) (OtherBodyIndex :type Integer) (bFromSweep :type Boolean) (SweepResult :type Hit%20Result%20Structure%20%28by%20ref%29))
  (Utilities|IsPlayer OtherActor
    (:IsPlayer
      (CallFunction|GetCrystalLocation)
      (CallFunction|GetCrystalScale)
      (CallFunction|GetLightIntensity)
      (bind (_direction _smoothlerpalpha _scale _lightintensity) (Timeline|TL_BlendAlpha Play)
        (:Update
          (CallFunction|TakeCrystaltoPlayer _smoothlerpalpha)
          (CallFunction|SetCrystalSmall _scale)
          (CallFunction|SetLightIntensity _lightintensity))
        (:Finished
          (Actor|DestroyActor))))))

(event EventBeginPlay)

(event Collision|EventActorBeginOverlap
  (params (OtherActor :type Actor%20Object%20Reference)))

(event EventTick
  (params (DeltaSeconds :type Float%20%28single-precision%29))
  (CallFunction|RotateActor))

(fn ConstructionScript)

(fn TakeCrystaltoPlayer
  (params (Alpha :type Float%20%28single-precision%29))
  (Transformation|SetActorLocation (Math|Vector|Lerp(Vector) (Variables|Default|GetLerpStartLocation) (Transformation|GetActorLocation (Game|Player|GetPlayerPawn 0)) Alpha) false false))

(fn GetCrystalLocation
  (Variables|Default|SetLerpStartLocation (Transformation|GetActorLocation)))

(fn GetCrystalScale
  (Variables|Default|SetLerpStartScale (Transformation|GetActorScale3D)))

(fn SetCrystalSmall
  (params (Alpha :type Float%20%28single-precision%29))
  (Transformation|SetActorScale3D (Math|Vector|Lerp(Vector) (Variables|Default|GetLerpStartScale) "0, 0, 0" Alpha)))

(fn GetLightIntensity
  (Variables|Default|SetLerpStartPointLightIntensity (Variables|/Script/Engine.LightComponentBase|GetIntensity (Variables|Default|GetPointLight))))

(fn SetLightIntensity
  (params (Alpha :type Float%20%28single-precision%29))
  (Rendering|Components|Light|SetIntensity (Variables|Default|GetPointLight) (Math|Float|Lerp (Variables|Default|GetLerpStartPointLightIntensity) 0.0 Alpha)))

(fn RotateActor
  (bind _returnvalue (Transformation|GetActorRotation))
  (Transformation|SetActorRotation (Math|Rotator|MakeRotator (.roll _returnvalue) (.pitch _returnvalue) (+ (.yaw _returnvalue) 1.0))))