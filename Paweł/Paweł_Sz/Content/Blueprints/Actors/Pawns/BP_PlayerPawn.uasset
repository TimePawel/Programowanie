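; Player pawn moved by physics torque, likely a rolling body, that restarts the level when damaged.
; Both movement axis inputs share one acceleration-based torque call on X and Y, scaled by a strength variable.
; Any damage calls ResetLevel, which fades the camera out, waits for the fade to finish, then reopens the current level.
; Escape quits the game.
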(event EventBeginPlay)

(event Collision|EventActorBeginOverlap
  (params (OtherActor :type Actor%20Object%20Reference)))

(event EventTick
  (params (DeltaSeconds :type Float%20%28single-precision%29)))

(event Game|Damage|EventAnyDamage
  (params (Damage :type Float%20%28single-precision%29) (DamageType :type Damage%20Type%20Object%20Reference) (InstigatedBy :type Controller%20Object%20Reference) (DamageCauser :type Actor%20Object%20Reference))
  (Utilities|ResetLevel))

(event Input|AxisEvents|InputAxisMoveForward/Backwards
  (params (AxisValue :type Float%20%28single-precision%29))
  (bind _torque_strenght (Variables|Default|GetTorque%20Strenght))
  (Class|PrimitiveComponent|AddTorqueinRadians (Variables|Default|GetPawn) (Math|Vector|MakeVector (* (stale Input|AxisEvents|InputAxisMoveLeft/Righ AxisValue) _torque_strenght) (* AxisValue _torque_strenght) 0.0) "None" true))

(event Input|AxisEvents|InputAxisMoveLeft/Righ
  (params (AxisValue :type Float%20%28single-precision%29))
  (bind _torque_strenght (Variables|Default|GetTorque%20Strenght))
  (Class|PrimitiveComponent|AddTorqueinRadians (Variables|Default|GetPawn) (Math|Vector|MakeVector (* AxisValue _torque_strenght) (* (stale Input|AxisEvents|InputAxisMoveForward/Backwards AxisValue) _torque_strenght) 0.0) "None" true))

(event Input|KeyboardEvents|Escape
  (params (Key :type Key%20Structure))
  (:Pressed
    (Game|QuitGame 0 "Quit")))

(fn ConstructionScript)